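; Enemy spawner actor for the wave system that spawns enemies at its own transform when GM_Core signals they can spawn.
; A looping timer, with its 3–6 second interval randomized once at start, draws from the ToSpawn list of enemy classes and counts.
; SelectEnemy favors larger remaining counts, re-rolling per entry, and decrements the pick.
; When all counts reach zero, the timer clears and SpawningDone becomes true.
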(event `self.ReceiveBeginPlay`
  (bind _asgm_core (cast `/Game/ForgottenTeasure/CoreClass/GM_Core` (`GameplayStatics.GetGameMode`)))
  (bind _output_get (set `self.GM_Core` _asgm_core))
  (add `/Game/ForgottenTeasure/CoreClass/GM_Core.CanSpawnEnemies` _output_get (delegate `SpawnEnemies`))
  (set `self.SpawningDone` false))

(event `SpawnEnemies`
  (bind _returnvalue (`KismetSystemLibrary.K2_SetTimerDelegate` (delegate `Spawn`) (`KismetMathLibrary.RandomFloatInRange` 3.0 6.0) true))
  (set `self.SpawnHandler` _returnvalue))

(event `Spawn`
  (if (not (== (`self.EnemiesAmount`) 0))
    (bind _enemy (`self.SelectEnemy`))
    (bind _returnvalue (`|SpawnActorFromClass` _enemy (`self.GetTransform`) "Undefined" "MultiplyWithRoot" null null))
    (`Pawn.SpawnDefaultController` (`Actor.Instigator` _returnvalue))
    (else
      (`KismetSystemLibrary.K2_ClearAndInvalidateTimerHandle` (`self.SpawnHandler`))
      (set `self.SpawningDone` true))))

(fn `EnemiesAmount`
  (returns (EnemiesAmount :type Integer))
  (locals (Sum :type Integer))
  (for _array_element (`self.ToSpawn`)
    (set `local.Sum` (+ (break `/Game/ForgottenTeasure/WaveSystem/ST_WaveData` _array_element) (`local.Sum`))))
  (return (`local.Sum`)))

(fn `SelectEnemy`
  (returns (Enemy :type "Actor Class Reference"))
  (locals (WaveData :type "/Game/ForgottenTeasure/WaveSystem/ST_WaveData Structure") (index :type Integer) (EnemiesSum :type Integer))
  (bind _wavedata_amount (break `/Game/ForgottenTeasure/WaveSystem/ST_WaveData` (`local.WaveData`)))
  (bind _wavedata_amount_2 (break `/Game/ForgottenTeasure/WaveSystem/ST_WaveData` (`local.WaveData`)))
  (bind (_wavedata_amount_3 _wavedata_enemy) (break `/Game/ForgottenTeasure/WaveSystem/ST_WaveData` (`local.WaveData`)))
  (bind (_wavedata_amount_4 _wavedata_enemy_2) (break `/Game/ForgottenTeasure/WaveSystem/ST_WaveData` (`local.WaveData`)))
  (for (_array_element _array_index) (`self.ToSpawn`)
    (set `local.WaveData` _array_element)
    (set `local.index` _array_index)
    (bind _output_get (set `local.EnemiesSum` (+ _wavedata_amount (`local.EnemiesSum`))))
    (if (>= _output_get (`KismetMathLibrary.RandomIntegerInRange` 1 (`self.EnemiesAmount`)))
      (bind _result (`/Engine/EditorBlueprintResources/StandardMacros.DecrementInt` _wavedata_amount_2)
        (:`  `
          (`KismetArrayLibrary.Array_Set` (`self.ToSpawn`) (`local.index`) (make `/Game/ForgottenTeasure/WaveSystem/ST_WaveData` _result _wavedata_enemy))
          (break)))))
  (set `local.EnemiesSum` 0)
  (return _wavedata_enemy_2))

(fn `UserConstructionScript`)
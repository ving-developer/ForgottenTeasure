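; Enemy character that takes damage, dies as a ragdoll and may drop a gold coin.
; AnyDamage clamps health while alive; sword hits also stop the attack montage and play a flinch, calling ReadyToChase on blend-out.
; At zero health it turns the mesh into a physics ragdoll, disables capsule collision and movement, rolls for a BP_GoldCoin, calls IsDeath and destroys itself after a delay.
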(event `self.ReceiveAnyDamage`
  (params (Damage :type "Float (single-precision)") (DamageType :type "DamageType Object Reference") (InstigatedBy :type "Controller Object Reference") (DamageCauser :type "Actor Object Reference"))
  ; Aplica dano a instância do inimigo caso ainda esteja vivo (IsAlive==true), configurando para que a vida dele não ultrapasse o MaxHealth e nem seja valor negativo. Quando chegar a zero a vida do inimigo define a variavel IsAlive como false  e chama o evento de morte
  (if (`self.IsAlive`)
    (bind _output_get (set `self.Health` (`KismetMathLibrary.FClamp` (- (`self.Health`) Damage) 0.0 (`self.MaxHealth`))))
    (if (== (`GameplayStatics.GetObjectClass` DamageCauser) "/Game/ForgottenTeasure/Player/BP_Sword.BP_Sword_C")
      (`AnimInstance.Montage_Stop` (`SkeletalMeshComponent.GetAnimInstance` (`self.Mesh`)) 0.0 "/Game/ForgottenTeasure/Enemy/Animations/Corpse_Attack_Montage.Corpse_Attack_Montage")
      (`|PlayMontage` (`self.Mesh`) "/Game/ForgottenTeasure/Enemy/Animations/Corpse_Flinch_back_Montage.Corpse_Flinch_back_Montage" 1.0 0.0 "None" false
        (:`then`
          (if (== _output_get 0.0) :!label _label
            (set `self.IsAlive` false)
            (`self.RagdollFunction`)
            (`self.DropCoin`)
            (`self.IsDeath`)
            (`KismetSystemLibrary.Delay` 5.0)
            (`self.K2_DestroyActor`)))
        (:`OnBlendOut`
          (`self.ReadyToChase`)))
      (else
        (goto _label)))))

(event `DropCoin`
  ; Evento chamado após o inimigo morrer, faz uma lógica de 50% de chance de spawnar uma moeda de ouro na localização em que o inimigo estava
  (if (`KismetMathLibrary.RandomBoolWithWeight` 0.5)
    (`|SpawnActorFromClass` "/Game/ForgottenTeasure/Assets/BP_GoldCoin.BP_GoldCoin_C" (`self.GetTransform`) "Undefined" "MultiplyWithRoot" null null)))

(fn `RagdollFunction`
  ; Evento de morte do inimigo, que desabilita a colisão da capsula, e dispara um evento de física na mesh do inimigo, fazendo com que o esqueleto dele se desmonte e caia no chão
  (`PrimitiveComponent.SetCollisionEnabled` (`self.CapsuleComponent`) "NoCollision")
  (`PrimitiveComponent.SetCollisionEnabled` (`self.Mesh`) "QueryAndPhysics")
  (`PrimitiveComponent.SetSimulatePhysics` (`self.Mesh`) true)
  (`MovementComponent.StopMovementImmediately` (`self.CharacterMovement`))
  (`CharacterMovementComponent.DisableMovement` (`self.CharacterMovement`)))

(fn `UserConstructionScript`)
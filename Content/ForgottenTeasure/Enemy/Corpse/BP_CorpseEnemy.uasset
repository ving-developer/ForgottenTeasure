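; BP_CorpseEnemy is a skeleton enemy derived from BP_DefaultEnemy that damages the player with sword swings.
; Montage-driven Attack and StopTrace events start and clear a looping timer that line-traces between two sword sockets.
; The player hit is stored and ignored by later traces until StopTrace resets it, limiting damage to once per swing.
; On possession it binds the parent's IsDeath dispatcher to silence its growl and play a falling-bones sound.
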(event `Stop Trace`
  ; Este evento está configurado para ser chamado no fim da animação de ataque no Corpse_Attack_Montage e ele invalida a variável TimeHandler fazendo com que Start Trace deixe de executar e reseta a variável PlayerAlreadyHitted que indica o jogador acertado por este ataque
  (`KismetSystemLibrary.K2_ClearAndInvalidateTimerHandle` (`self.TimeHandler`))
  (set `self.PlayerAlreadyHitted` null))

(event `Attack`
  ; Este evento é chamado no início da animação de ataque através do Corpse_Attack_Montage e ele executa a cada poucos milisegundos o evento StartTrace enquanto a variável TimeHandler não for invalidada pelo evento StopTrace
  (bind _returnvalue (`KismetSystemLibrary.K2_SetTimerDelegate` (delegate `Start Trace`) 0.01 true))
  (set `self.TimeHandler` _returnvalue))

(event `Start Trace`
  (bind _sword (`self.Sword`))
  ; Desenha linhas de trace conforme a posição atual da espada do Inimigo, utilizando os sockets criados no mesh da Sword. Essas linhas verificam em tempo real se a espada passou pela capsula de colisão do BP_Player
  (bind _outhit (`KismetSystemLibrary.LineTraceSingle` (`SceneComponent.GetSocketLocation` _sword "TrailStartSocket") (`SceneComponent.GetSocketLocation` _sword "TrailEndSocket") "TraceTypeQuery1" false (`|MakeArray` (`self.PlayerAlreadyHitted`)) "None" true (struct :`R` 1.0 :`A` 1.0) (struct :`G` 1.0 :`A` 1.0) 1.0))
  (bind (_bblockinghit _binitialoverlap _time _distance _location _impactpoint _normal _impactnormal _physmat _hitactor) (`GameplayStatics.BreakHitResult` _outhit))
  ; Quando um hit acerta o Player, essa lógica verifica se a classe do objeto acertado é BP_Player, caso seja, preenche a variável PlayerAlreadyHitted com o valor do HitActor (BP_Player) e após isso executa a ação de ApplyDamage no jogador. PlayerAlreadyHitted é utilizado em outro ponto para indicar que alguma outra linha de trace já acertou o inimigo e portanto as próximas linhas não podem aplicar novos danos no jogador
  (if (== (`GameplayStatics.GetObjectClass` _hitactor) "/Game/ForgottenTeasure/Player/BP_Player.BP_Player_C")
    (set `self.PlayerAlreadyHitted` _hitactor)
    (`GameplayStatics.ApplyDamage` _hitactor 25.0)))

(event `self.ReceivePossessed`
  (params (NewController :type "Controller Object Reference"))
  ; Assim que essa classe de BluePrint toma posse da instância do inimigo (EventPossessed), passa a escutar o Event Dispatcher "IsDeath" criado na classe pai BP_DefaultEnemy, e assim que ele for chamado executa IsDeath_Event, que por sua vez desabilita o som default do CorpseEnemy e executa o som de morte dele
  (add `self.IsDeath` (delegate `IsDeath_Event`)))

(event `IsDeath_Event`
  ; Assim que essa classe de BluePrint toma posse da instância do inimigo (EventPossessed), passa a escutar o Event Dispatcher "IsDeath" criado na classe pai BP_DefaultEnemy, e assim que ele for chamado executa IsDeath_Event, que por sua vez desabilita o som default do CorpseEnemy e executa o som de morte dele
  (`ActorComponent.SetActive` (`self.Skeleton Growl`) false false)
  (`GameplayStatics.PlaySoundAtLocation` "/Game/ForgottenTeasure/Enemy/Sounds/fallingBones_Cue.fallingBones_Cue" (`self.K2_GetActorLocation`) (struct) 1.0 1.0 0.0 null null null null))

(fn `UserConstructionScript`
  (`parent.UserConstructionScript`))
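; Explosive barrel actor that detonates 0.1 seconds after receiving any damage.
; The explosion applies radial damage around itself, ignoring itself, fires a RadialForce impulse, plays sound and particle effects, then destroys the actor.
; Because any damage triggers it, the blast can set off other barrels of this class within range.
; A disconnected debug sphere node can visualize the damage radius.
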(event `self.ReceiveAnyDamage`
  (params (Damage :type "Float (single-precision)") (DamageType :type "DamageType Object Reference") (InstigatedBy :type "Controller Object Reference") (DamageCauser :type "Actor Object Reference"))
  (`KismetSystemLibrary.Delay` 0.1)
  (`GameplayStatics.ApplyRadialDamage` 50.0 (`self.K2_GetActorLocation`) (`self.radiusRange`) null (`|MakeArray` self) null null)
  (`RadialForceComponent.FireImpulse` (`self.RadialForce`))
  (`GameplayStatics.PlaySoundAtLocation` "/Game/ForgottenTeasure/Assets/Barrel/BarrelExplosion.BarrelExplosion" (`self.K2_GetActorLocation`) (struct) 1.0 1.0 0.0 null null null null)
  (`GameplayStatics.SpawnEmitterAtLocation` "/Game/Realistic_Starter_VFX_Pack_Vol2/Particles/Explosion/P_Explosion_Big_A.P_Explosion_Big_A" (`self.K2_GetActorLocation`))
  (`self.K2_DestroyActor`))

(fn `UserConstructionScript`)